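; Base dungeon character Blueprint that handles sprite-based damage reactions and invincibility recovery.
; AnyDamage checks and reduces health through BPCHealth, then plays a sound, timeline-driven knockback away from the causer and a red sprite flash.
; It calls an empty HandleHitExtended hook, then freezes an attacking dungeon character briefly via CustomTimeDilation hit stop.
; When BPCHealth reports invincibility expired, it clears the flicker timer, shows the sprite and re-enables HurtBox queries.
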(event Custom|OnInvinsibilityExpired
  (Utilities|Time|ClearandInvalidateTimerbyHandle (Variables|Default|GetFlickerHandle))
  (Rendering|SetVisibility (Variables|Default|GetSprite) true false)
  (Collision|SetCollisionEnabled (Variables|Default|GetHurtBox) "QueryOnly"))

(event Custom|FlashSprite
  (Sprite|SetSpriteColor (Variables|Default|GetSprite) "(R=1.000000,G=0.029373,B=0.000000,A=1.000000)")
  (Utilities|FlowControl|RetriggerableDelay (Variables|Default|GetFlashDuration))
  (Sprite|SetSpriteColor (Variables|Default|GetSprite) "(R=1.000000,G=1.000000,B=1.000000,A=1.000000)"))

(event Custom|HitStop
  (Variables|Default|SetCustomTimeDilation 0.0)
  (Utilities|FlowControl|RetriggerableDelay (Variables|Default|GetHitstopDuration))
  (Variables|Default|SetCustomTimeDilation 1.0))

(event Custom|GetKnockback
  (params (Attacker :type Actor%20Object%20Reference))
  (Components|Timeline|SetPlayRate (Variables|Default|GetKnockbackTimeline) 5.0)
  (Variables|Default|SetKnockbackDirection (Math|Vector|GetForwardVector (Math|Rotator|FindLookatRotation (Transformation|GetActorLocation Attacker) (Transformation|GetActorLocation))))
  (Timeline|KnockbackTimeline PlayFromStart
    (:Update
      (Variables|/Script/Engine.MovementComponent|SetVelocity (Variables|Character|GetCharacterMovement) (* (Variables|Default|GetKnockbackDirection) (Variables|Default|GetKnockbackStrength) (Utilities|Time|GetWorldDeltaSeconds))))))

(event Game|Damage|EventAnyDamage
  (params (Damage :type Float%20%28single-precision%29) (DamageType :type Damage%20Type%20Object%20Reference) (InstigatedBy :type Controller%20Object%20Reference) (DamageCauser :type Actor%20Object%20Reference))
  (if (Default|CanbeDamaged (Variables|Default|GetBPC_Health))
    (Default|DecreaseHealth (Variables|Default|GetBPC_Health) Damage)
    (Audio|PlaySound2D (Variables|Default|GetHitSound) 1.0 1.0 0.0 0 0)
    (CallFunction|GetKnockback DamageCauser)
    (CallFunction|FlashSprite)
    (CallFunction|HandleHitExtended)
    (bind _asbp_dungeon_char_base (Utilities|Casting|CastToBP_DungeonChar_Base DamageCauser))
    (CallFunction|HitStop _asbp_dungeon_char_base)))

(event EventBeginPlay
  (EventDispatchers|BindEventtoInvinsibilityExpired (Variables|Default|GetBPC_Health) (delegate Custom|OnInvinsibilityExpired)))

(fn ConstructionScript)

(fn HandleHitExtended)

(fn SetSpriteVisbility
  (bind _sprite (Variables|Default|GetSprite))
  (Rendering|SetVisibility _sprite (not (Variables|/Script/Engine.SceneComponent|GetbVisible _sprite)) false))