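; Health component that tracks an owner's current health, defeated state and temporary invincibility, starting at max health on BeginPlay.
; DecreaseHealth and IncreaseHealth clamp the value between zero and max, with only damage updating the defeated flag.
; SetInvinsibility uses a retriggerable delay, so repeat calls restart the window before InvinsibilityExpired is called.
; CanBeDamaged combines both flags, but DecreaseHealth does not check it itself.
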(event Custom|SetInvinsibility
  (Variables|Default|SetIsInvincible true)
  (Utilities|FlowControl|RetriggerableDelay (Variables|Default|GetInvinsibilityDuration))
  (Variables|Default|SetIsInvincible false)
  (Default|CallInvinsibilityExpired))

(event EventBeginPlay
  (Variables|Default|SetCurrentHealth (Variables|Default|GetMaxHealth)))

(event EventTick
  (params (DeltaSeconds :type Float%20%28single-precision%29)))

(fn DecreaseHealth
  (params (Damage :type Float%20%28double-precision%29))
  (bind _output_get (Variables|Default|SetCurrentHealth (Math|Float|Max(Float) (- (Variables|Default|GetCurrentHealth) Damage) 0.0)))
  (Variables|Default|SetIsDefeated (<= _output_get 0.0)))

(fn CanbeDamaged
  (return (and (not (Variables|Default|GetIsDefeated)) (not (Variables|Default|GetIsInvincible)))))

(fn IncreaseHealth
  (params (IncreaseAmount :type Float%20%28double-precision%29))
  (Variables|Default|SetCurrentHealth (Math|Float|Min(Float) (+ IncreaseAmount (Variables|Default|GetCurrentHealth)) (Variables|Default|GetMaxHealth))))