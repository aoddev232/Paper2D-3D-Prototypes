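; Player character Red for a top-down game, with flipbook sprite animation, Enhanced Input movement and interaction.
; BeginPlay adds the input mapping context and creates the main HUD widget.
; Move input drives world-axis movement and stores direction, which selects walk or idle flipbooks, horizontal taking priority.
; Interact shows the message from the first overlapping BPI_Interact actor on the HUD, hiding it after a retriggerable delay.
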(event Input|EnhancedActionEvents|EnhancedInputActionIA_Move
  (params (ActionValue :type Vector%202D%20Structure) (ElapsedSeconds :type Float%20%28double-precision%29) (TriggeredSeconds :type Float%20%28double-precision%29) (InputAction :type Input%20Action%20Object%20Reference :default "/Game/Input/Actions/IA_Move.IA_Move"))
  (bind (_x _y) (Math|Vector2D|BreakVector2D ActionValue))
  (:Triggered
    (Variables|Default|SetDirectionality ActionValue)
    (Pawn|Input|AddMovementInput "1.0,0.0,0.0" _x false)
    (Pawn|Input|AddMovementInput "0.000000,1.000000,0.000000" _y false)
    (CallFunction|UpdateAnimation false))
  (:Completed
    (CallFunction|UpdateAnimation true)))

(event Input|EnhancedActionEvents|EnhancedInputActionIA_Interact
  (params (ActionValue :type Boolean) (ElapsedSeconds :type Float%20%28double-precision%29) (TriggeredSeconds :type Float%20%28double-precision%29) (InputAction :type Input%20Action%20Object%20Reference :default "/Game/Input/Actions/IA_Interact.IA_Interact"))
  (bind _array_element (Utilities|Array|ForEachLoopwithBreak (Collision|GetOverlappingActors (Variables|Default|GetInteractCheck) 0 :!class /Script/Engine.PrimitiveComponent) :!label _label)
    (:LoopBody
      (if (Utilities|DoesObjectImplementInterface _array_element "/Game/Blueprints/Interfaces/BPI_Interact.BPI_Interact_C")
        (bind _text (Class|BPIInteract|Interact(Message) _array_element))
        (Default|SetDialogueText (Variables|Default|GetMainHUD) _text)
        (goto _label Break)))
    (:Completed
      (Utilities|FlowControl|RetriggerableDelay (Variables|Default|GetHideMessageDelay))
      (Default|HideMessage (Variables|Default|GetMainHUD)))))

(event EventBeginPlay
  (Utilities|FlowControl|Sequence
    (:then_0
      (bind _asplayer_controller (Utilities|Casting|CastToPlayerController (Pawn|GetController)))
      (Input|AddMappingContext (PlayerController|LocalPlayerSubsystems|GetEnhancedInputLocalPlayerSubsystem _asplayer_controller) "/Game/Input/IMC_TopDown.IMC_TopDown" 0 "(bIgnoreAllPressedKeysUntilRelease=True,bForceImmediately=False,bNotifyUserSettings=False)"))
    (:then_1
      (bind _returnvalue (UserInterface|CreateWidget "/Game/Widgets/WBP_MainHUD.WBP_MainHUD_C"))
      (bind _output_get (Variables|Default|SetMainHUD _returnvalue))
      (UserInterface|Viewport|AddtoViewport _output_get 0))))

(fn ConstructionScript)

(fn UpdateAnimation
  (params (TransitionToIdle :type Boolean))
  (if TransitionToIdle
    (Math|Float|CompareFloat (.X (Math|Vector2D|BreakVector2D (Variables|Default|GetDirectionality))) 0.0
      (:>
        (Sprite|SetFlipbook (Variables|Default|GetSprite) "/Game/PaperAssets/Characters/Red/FB_Red_Idle_Right.FB_Red_Idle_Right"))
      (:==
        (Math|Float|CompareFloat (.Y (Math|Vector2D|BreakVector2D (Variables|Default|GetDirectionality))) 0.0
          (:>
            (Sprite|SetFlipbook (Variables|Default|GetSprite) "/Game/PaperAssets/Characters/Red/FB_Red_Idle_Downward.FB_Red_Idle_Downward"))
          (:<
            (Sprite|SetFlipbook (Variables|Default|GetSprite) "/Game/PaperAssets/Characters/Red/FB_Red_Idle_Up.FB_Red_Idle_Up"))))
      (:<
        (Sprite|SetFlipbook (Variables|Default|GetSprite) "/Game/PaperAssets/Characters/Red/FB_Red_Idle_Left.FB_Red_Idle_Left")))
    (else
      (Math|Float|CompareFloat (.X (Math|Vector2D|BreakVector2D (Variables|Default|GetDirectionality))) 0.0
        (:>
          (Sprite|SetFlipbook (Variables|Default|GetSprite) "/Game/PaperAssets/Characters/Red/FB_Red_Walk_Right.FB_Red_Walk_Right"))
        (:==
          (Math|Float|CompareFloat (.Y (Math|Vector2D|BreakVector2D (Variables|Default|GetDirectionality))) 0.0
            (:>
              (Sprite|SetFlipbook (Variables|Default|GetSprite) "/Game/PaperAssets/Characters/Red/FB_Red_Walk_Downward.FB_Red_Walk_Downward"))
            (:<
              (Sprite|SetFlipbook (Variables|Default|GetSprite) "/Game/PaperAssets/Characters/Red/FB_Red_Walk_Upward.FB_Red_Walk_Upward"))))
        (:<
          (Sprite|SetFlipbook (Variables|Default|GetSprite) "/Game/PaperAssets/Characters/Red/FB_Red_Walk_Left.FB_Red_Walk_Left"))))))